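; Spaceship pawn Blueprint that puts a ship HUD on screen and exposes flight telemetry.
; On BeginPlay it creates W_ShipHUD for its PlayerController and adds it to the viewport.
; GetWidgetTelemetryData passes through pitch, yaw, roll, control power and max velocity values from the SpaceshipGenMovement component.
; The acceleration telemetry, control limit and IsAccelerating functions are stubs returning zero or false.
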(event EventBeginPlay
  (|CallParentFunction)
  (bind _asplayer_controller (Utilities|Casting|CastToPlayerController (Pawn|GetController)))
  (bind _returnvalue (UserInterface|CreateWidget "/Game/SpaceshipPlugin/Widgets/HUD_Ship/W_ShipHUD.W_ShipHUD_C" _asplayer_controller))
  (UserInterface|Viewport|AddtoViewport _returnvalue 0))

(fn ConstructionScript)

(fn GetWidgetTelemetryData
  (bind _spaceshipgenmovement (Variables|Default|GetSpaceshipGenMovement))
  (return (Variables|/Script/SpaceshipMovement.SpaceshipGenMovementComponent|GetCurrentPitch _spaceshipgenmovement) (Variables|/Script/SpaceshipMovement.SpaceshipGenMovementComponent|GetCurrentYaw _spaceshipgenmovement) (Variables|/Script/SpaceshipMovement.SpaceshipGenMovementComponent|GetDesiredPitch _spaceshipgenmovement) (Variables|/Script/SpaceshipMovement.SpaceshipGenMovementComponent|GetDesiredYaw _spaceshipgenmovement) (Variables|/Script/SpaceshipMovement.SpaceshipGenMovementComponent|GetMaxVelocity _spaceshipgenmovement) (Variables|/Script/SpaceshipMovement.SpaceshipGenMovementComponent|GetDesiredRoll _spaceshipgenmovement) (Variables|/Script/SpaceshipMovement.SpaceshipGenMovementComponent|GetPitchControlPower _spaceshipgenmovement) (Variables|/Script/SpaceshipMovement.SpaceshipGenMovementComponent|GetYawControlPower _spaceshipgenmovement) (Variables|/Script/SpaceshipMovement.SpaceshipGenMovementComponent|GetRollControlPower _spaceshipgenmovement)))

(fn GetAccelerationTelemetry
  (return "0, 0, 0"))

(fn GetControlLimits
  (return 0.0 0.0 0.0))

(fn IsAccelerating
  (return false))